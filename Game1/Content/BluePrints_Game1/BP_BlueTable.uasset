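; BP_BlueTable is a colour-matching puzzle table that checks which BP_Lv3Cube is placed on it.
; When a cube enters its Box, a "blue" tag sets the BlueStatue flag, while any other cube teleports the first BP_FirstPersonCharacter to the first BP_TeleportPoint02.
; Any end overlap on the Box clears the flag, regardless of which actor leaves.
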(event `self.Box.OnComponentBeginOverlap`
  (params (OverlappedComponent :type "PrimitiveComponent Object Reference") (OtherActor :type "Actor Object Reference") (OtherComp :type "PrimitiveComponent Object Reference") (OtherBodyIndex :type Integer) (bFromSweep :type Boolean) (SweepResult :type "HitResult Structure (by ref)"))
  (bind _asbp_lv_3cube (cast `/Game/BluePrints_Game1/BP_Lv3Cube` OtherActor))
  (if (`self.ActorHasTag` _asbp_lv_3cube "blue")
    (set `self.BlueStatue` true)
    (`KismetSystemLibrary.PrintString` "Blue")
    (else
      (bind _outactors (`GameplayStatics.GetAllActorsOfClass` "/Game/BluePrints_Game1/BP_TeleportPoint02.BP_TeleportPoint02_C"))
      (bind _outactors_2 (`GameplayStatics.GetAllActorsOfClass` "/Game/FirstPerson/Blueprints/BP_FirstPersonCharacter.BP_FirstPersonCharacter_C"))
      (bind (_returnvalue_location _returnvalue_rotation) (`KismetMathLibrary.BreakTransform` (`SceneComponent.K2_GetComponentToWorld` (`Actor.RootComponent` (`|GetArrayItem` _outactors)))))
      (`self.K2_TeleportTo` (`|GetArrayItem` _outactors_2) _returnvalue_location _returnvalue_rotation))))

(event `self.Box.OnComponentEndOverlap`
  (params (OverlappedComponent :type "PrimitiveComponent Object Reference") (OtherActor :type "Actor Object Reference") (OtherComp :type "PrimitiveComponent Object Reference") (OtherBodyIndex :type Integer))
  (set `self.BlueStatue` false))

(fn `UserConstructionScript`)