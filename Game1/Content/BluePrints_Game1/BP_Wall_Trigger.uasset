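; BP_Wall_Trigger is a trigger volume that tips over a wall once two other triggers are both active.
; On box overlap, it loops over the entering actor's overlaps and checks the In flags of the first BP_Trigger01 and BP_Trigger02 found in the level.
; If both are set, it slows the first BP_Wall's OpenWallT timeline and plays its own timeline, lerping that wall's root pitch to -90 degrees.
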(event `self.Box.OnComponentBeginOverlap`
  (params (OverlappedComponent :type "PrimitiveComponent Object Reference") (OtherActor :type "Actor Object Reference") (OtherComp :type "PrimitiveComponent Object Reference") (OtherBodyIndex :type Integer) (bFromSweep :type Boolean) (SweepResult :type "HitResult Structure (by ref)"))
  (for _ (`self.GetOverlappingActors` OtherActor "/Script/Engine.Actor")
    (bind _outactors (`GameplayStatics.GetAllActorsOfClass` "/Game/BluePrints_Game1/BP_Trigger01.BP_Trigger01_C"))
    (bind _outactors_2 (`GameplayStatics.GetAllActorsOfClass` "/Game/BluePrints_Game1/BP_Trigger02.BP_Trigger02_C"))
    (if (and (`/Game/BluePrints_Game1/BP_Trigger02.In?` (`|GetArrayItem` _outactors_2)) (`/Game/BluePrints_Game1/BP_Trigger01.In?` (`|GetArrayItem` _outactors)))
      (bind _outactors_3 (`GameplayStatics.GetAllActorsOfClass` "/Game/BluePrints_Game1/BP_Wall.BP_Wall_C"))
      (bind _output (`|GetArrayItem` _outactors_3))
      (`TimelineComponent.SetPlayRate` (`/Game/BluePrints_Game1/BP_Wall.Open Wall T` _output) (/ 1.0 5.0))
      (bind (_direction _wall_track) (`Timeline|Timeline`)
        (:`Update`
          (`SceneComponent.K2_SetRelativeRotation` (`Actor.RootComponent` _output) (`KismetMathLibrary.MakeRotator` 0.0 (`KismetMathLibrary.Lerp` 0.0 -90.0 _wall_track)) false false)
          (break))))))

(fn `UserConstructionScript`)