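; BP_LV2Trigger is a level 2 trigger that tips a wall over once the letter puzzle (A, P, S, S2) is solved.
; On box overlap it finds the four letter actors by class and checks that all their flags are true.
; If so, a slowed timeline lerps the pitch of the first BP_WallLv2 from 0 to -90 degrees.
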(event `self.Box.OnComponentBeginOverlap`
  (params (OverlappedComponent :type "PrimitiveComponent Object Reference") (OtherActor :type "Actor Object Reference") (OtherComp :type "PrimitiveComponent Object Reference") (OtherBodyIndex :type Integer) (bFromSweep :type Boolean) (SweepResult :type "HitResult Structure (by ref)"))
  (bind _outactors (`GameplayStatics.GetAllActorsOfClass` "/Game/BluePrints_Game1/BP_LetterA.BP_LetterA_C"))
  (bind _outactors_2 (`GameplayStatics.GetAllActorsOfClass` "/Game/BluePrints_Game1/BP_LetterP.BP_LetterP_C"))
  (bind _outactors_3 (`GameplayStatics.GetAllActorsOfClass` "/Game/BluePrints_Game1/BP_LetterS.BP_LetterS_C"))
  (bind _outactors_4 (`GameplayStatics.GetAllActorsOfClass` "/Game/BluePrints_Game1/BP_LetterS2.BP_LetterS2_C"))
  (if (and (`/Game/BluePrints_Game1/BP_LetterS2.S2isTrue` (`|GetArrayItem` _outactors_4)) (and (`/Game/BluePrints_Game1/BP_LetterS.S1isTrue` (`|GetArrayItem` _outactors_3)) (and (`/Game/BluePrints_Game1/BP_LetterP.PisTrue` (`|GetArrayItem` _outactors_2)) (`/Game/BluePrints_Game1/BP_LetterA.AisTrue` (`|GetArrayItem` _outactors)))))
    (bind _outactors_5 (`GameplayStatics.GetAllActorsOfClass` "/Game/BluePrints_Game1/BP_WallLv2.BP_WallLv2_C"))
    (bind _output (`|GetArrayItem` _outactors_5))
    (`TimelineComponent.SetPlayRate` (`/Game/BluePrints_Game1/BP_WallLv2.Timeline` _output) (/ 1.0 5.0))
    (bind (_direction _wall_track) (`Timeline|Timeline`)
      (:`Update`
        (`SceneComponent.K2_SetRelativeRotation` (`Actor.RootComponent` _output) (`KismetMathLibrary.MakeRotator` 0.0 (`KismetMathLibrary.Lerp` 0.0 -90.0 _wall_track)) false false)))))

(fn `UserConstructionScript`)