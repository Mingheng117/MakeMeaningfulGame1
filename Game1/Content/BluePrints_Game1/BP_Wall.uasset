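; BP_Wall is an interactable wall that swings open and closed by rotating its WallLv1 component in pitch.
; Interact checks IsOpen, sets the timeline's play rate from the open or close duration, then triggers OpenWall or CloseWall.
; The OpenWallT timeline plays forward or in reverse to lerp pitch between ClosePosition and OpenPosition.
; IsOpen flips only when the timeline finishes, and Interact always returns false.
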(event `Open Wall`
  (bind (_direction _wall_track) (`Timeline|Open Wall T` :!label _label)
    (:`Update`
      (`SceneComponent.K2_SetRelativeRotation` (`self.Wall_Lv1`) (`KismetMathLibrary.MakeRotator` 0.0 (`KismetMathLibrary.Lerp` (`self.Close Position`) (`self.Open Position`) _wall_track)) false false))
    (:`Finished`
      (set `self.IsOpen?` (not (`self.IsOpen?`))))))

(event `Close Wall`
  (goto _label :!via `Reverse`))

(fn `Interact`
  (params (Interactor :type "Character Object Reference"))
  (returns (`Did Interact?` :type Boolean))
  (bind _open_wall_t (`self.Open Wall T`))
  (if (not (`self.IsOpen?`))
    (`TimelineComponent.SetPlayRate` _open_wall_t (/ 1.0 (`self.Time To Open (s)`)))
    (`self.Open Wall`)
    (else
      (`TimelineComponent.SetPlayRate` _open_wall_t (/ 1.0 (`self.Time To Close (s)`)))
      (`self.Close Wall`)))
  (return false))

(fn `UserConstructionScript`)